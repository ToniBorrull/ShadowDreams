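; Base inventory item actor that the player picks up, with hooks for throwing, locking and puzzles.
; Sphere overlap caches the first-person character and enables input, so E passes Iteminfo to PickItems and destroys the actor.
; Inner and outer collisions swap two billboards by player proximity.
; Events throw the mesh along camera forward, toggle the lock flag, spawn a puzzle unlocker in place, or disable a solved piece's collision and physics.
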(event OnComponentBeginOverlap(Sphere)
  (params (OverlappedComponent :type Primitive%20Component%20Object%20Reference) (OtherActor :type Actor%20Object%20Reference) (OtherComp :type Primitive%20Component%20Object%20Reference) (OtherBodyIndex :type Integer) (bFromSweep :type Boolean) (SweepResult :type Hit%20Result%20Structure%20%28by%20ref%29))
  (bind _asbp_first_person_character (Utilities|Casting|CastToBP_FirstPersonCharacter OtherActor))
  (Variables|Default|SetAs%20BP%20First%20Person%20Character _asbp_first_person_character)
  (Input|EnableInput (Game|GetPlayerController 0)))

(event OnComponentEndOverlap(Sphere)
  (params (OverlappedComponent :type Primitive%20Component%20Object%20Reference) (OtherActor :type Actor%20Object%20Reference) (OtherComp :type Primitive%20Component%20Object%20Reference) (OtherBodyIndex :type Integer))
  (Input|DisableInput (Game|GetPlayerController 0)))

(event OnComponentBeginOverlap(innerCollision)
  (params (OverlappedComponent :type Primitive%20Component%20Object%20Reference) (OtherActor :type Actor%20Object%20Reference) (OtherComp :type Primitive%20Component%20Object%20Reference) (OtherBodyIndex :type Integer) (bFromSweep :type Boolean) (SweepResult :type Hit%20Result%20Structure%20%28by%20ref%29))
  (if (== OtherActor (Game|GetPlayerCharacter 0))
    (Rendering|SetVisibility (Variables|Default|GetBillboard1) true false)
    (Rendering|SetVisibility (Variables|Default|GetBillboard) false false)))

(event OnComponentEndOverlap(innerCollision)
  (params (OverlappedComponent :type Primitive%20Component%20Object%20Reference) (OtherActor :type Actor%20Object%20Reference) (OtherComp :type Primitive%20Component%20Object%20Reference) (OtherBodyIndex :type Integer))
  (if (== (Game|GetPlayerCharacter 0) OtherActor)
    (Rendering|SetVisibility (Variables|Default|GetBillboard1) false false)
    (Rendering|SetVisibility (Variables|Default|GetBillboard) true false)))

(event OnComponentBeginOverlap(outerCollision)
  (params (OverlappedComponent :type Primitive%20Component%20Object%20Reference) (OtherActor :type Actor%20Object%20Reference) (OtherComp :type Primitive%20Component%20Object%20Reference) (OtherBodyIndex :type Integer) (bFromSweep :type Boolean) (SweepResult :type Hit%20Result%20Structure%20%28by%20ref%29))
  (if (== OtherActor (Game|GetPlayerCharacter 0))
    (Rendering|SetVisibility (Variables|Default|GetBillboard) true false)))

(event OnComponentEndOverlap(outerCollision)
  (params (OverlappedComponent :type Primitive%20Component%20Object%20Reference) (OtherActor :type Actor%20Object%20Reference) (OtherComp :type Primitive%20Component%20Object%20Reference) (OtherBodyIndex :type Integer))
  (if (== OtherActor (Game|GetPlayerCharacter 0))
    (Rendering|SetVisibility (Variables|Default|GetBillboard) false false)))

(event Custom|SpawnPuzzleUnlocker
  (params (puzzlePiece :type BP%20Master%20Item%20Class%20Reference))
  (bind _returnvalue (Transformation|GetActorTransform))
  (Game|SpawnActorfromClass puzzlePiece (Math|Transform|MakeTransform (.location _returnvalue) (.rotation _returnvalue) "1.000000,1.000000,1.000000") "Undefined" "MultiplyWithRoot" 0 0))

(event Custom|LockItem
  (Variables|Default|SetitemIsLocked true))

(event Custom|UnlockItem
  (Variables|Default|SetitemIsLocked false))

(event Custom|PuzzlePieceSolved
  (Components|DestroyComponent (Variables|Default|GetBox))
  (Physics|SetSimulatePhysics (Variables|Default|GetitemMesh) false)
  (Collision|SetCollisionEnabled (Variables|Default|GetitemMesh) "NoCollision"))

(event EventBeginPlay)

(event Collision|EventActorBeginOverlap
  (params (OtherActor :type Actor%20Object%20Reference)))

(event EventTick
  (params (DeltaSeconds :type Float%20%28single-precision%29)))

(event EventThrowObject
  (Physics|SetPhysicsLinearVelocity (Variables|Default|GetitemMesh) (* (Math|Vector|GetForwardVector (Camera|GetCameraRotation (Variables|/Script/Engine.PlayerController|GetPlayerCameraManager (Game|GetPlayerController 0)))) 5e+02) true "None"))

(event EventSolvePuzzle
  (Development|PrintString "PuzzleSolved"))

(event Input|KeyboardEvents|E
  (params (Key :type Key%20Structure :default "None"))
  (:Pressed
    (Default|PickItems (Variables|Default|GetAs%20BP%20First%20Person%20Character) (Variables|Default|GetIteminfo))
    (Actor|DestroyActor)))

(fn ConstructionScript)