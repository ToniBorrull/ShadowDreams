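; BP_PlayerPosManager periodically teleports the first-person player character through a looping list of spawn positions.
; On BeginPlay it finds and caches the BP_FirstPersonCharacter.
; Tick accumulates a timer, and whenever it exceeds FaseTime it resets, advances the cycle index with wraparound, and moves the player to that SpawnPositions actor's location without sweeping.
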(event EventBeginPlay
  (bind _returnvalue (Actor|GetActorOfClass "/Game/Vertical/Player/BP_FirstPersonCharacter.BP_FirstPersonCharacter_C"))
  (Variables|Default|SetPlayer _returnvalue))

(event EventTick
  (params (DeltaSeconds :type Float%20%28single-precision%29))
  (Utilities|IsValid (Variables|Default|GetPlayer)
    (:Is%20Valid
      (Variables|Default|Settimer (+ DeltaSeconds (Variables|Default|Gettimer)))
      (if (> (Variables|Default|Gettimer) (Variables|Default|GetfaseTime))
        (Variables|Default|Settimer 0.0)
        (Math|Integer|IncrementInt (Variables|Default|Getcicle)
          (:%20%20
            (if (> (Variables|Default|Getcicle) (- (Utilities|Array|Length (Variables|Default|GetSpawnPositions)) 1))
              (Variables|Default|Setcicle 0))
            (Transformation|SetActorLocation (Variables|Default|GetPlayer) (Transformation|GetActorLocation (Utilities|Array|Get(acopy) (Variables|Default|GetSpawnPositions) (Variables|Default|Getcicle))) false true)))))))

(fn ConstructionScript)