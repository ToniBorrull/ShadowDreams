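; BP_FallenObjectsSpawn is a trigger box that returns fallen items to the player.
; BeginPlay caches the BP_FirstPersonCharacter as Player.
; When a BP_MasterItem overlaps the box, it spawns a fresh actor of the same class at the player's capsule location, then destroys the original and prints a debug message.
; The replacement is a new instance, as nothing copies the original's state.
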(event OnComponentBeginOverlap(Box)
  (params (OverlappedComponent :type Primitive%20Component%20Object%20Reference) (OtherActor :type Actor%20Object%20Reference) (OtherComp :type Primitive%20Component%20Object%20Reference) (OtherBodyIndex :type Integer) (bFromSweep :type Boolean) (SweepResult :type Hit%20Result%20Structure%20%28by%20ref%29))
  (Utilities|Casting|CastToBP_MasterItem OtherActor)
  (if true
    (Game|SpawnActorfromClass (Utilities|GetClass OtherActor) (Math|Conversions|ToTransform(Vector) (Transformation|GetWorldLocation (Variables|/Script/Engine.Character|GetCapsuleComponent (Variables|Default|Getplayer)))) "Undefined" "MultiplyWithRoot" 0 0)
    (Actor|DestroyActor OtherActor)
    (Development|PrintString "Actor destroyed")))

(event EventBeginPlay
  (bind _returnvalue (Actor|GetActorOfClass "/Game/Vertical/Player/BP_FirstPersonCharacter.BP_FirstPersonCharacter_C"))
  (Variables|Default|Setplayer _returnvalue))

(fn ConstructionScript)