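; BP_FinalPuzzle is a puzzle checker actor that accepts three specific item pieces, each in its own trigger.
; Check1, Check2 and Check3 compare an overlapping actor's exact class against PuzzlePiece1, PuzzlePiece2 and PuzzlePiece3 respectively.
; A match is cast to BP_MasterItem, teleported to that slot's scene component location, then receives LockItem and PuzzlePieceSolved.
; The blueprint itself tracks no overall completion; each slot works independently.
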(event OnComponentBeginOverlap(Check1)
  (params (OverlappedComponent :type Primitive%20Component%20Object%20Reference) (OtherActor :type Actor%20Object%20Reference) (OtherComp :type Primitive%20Component%20Object%20Reference) (OtherBodyIndex :type Integer) (bFromSweep :type Boolean) (SweepResult :type Hit%20Result%20Structure%20%28by%20ref%29))
  (if (== (Variables|Default|GetPuzzlePiece1) (Utilities|GetClass OtherActor))
    (bind _asbp_master_item (Utilities|Casting|CastToBP_MasterItem OtherActor))
    (Transformation|SetActorLocation _asbp_master_item (Transformation|GetWorldLocation (Variables|Default|GetScene2)) false true)
    (Default|LockItem _asbp_master_item)
    (Default|PuzzlePieceSolved _asbp_master_item)))

(event OnComponentBeginOverlap(Check2)
  (params (OverlappedComponent :type Primitive%20Component%20Object%20Reference) (OtherActor :type Actor%20Object%20Reference) (OtherComp :type Primitive%20Component%20Object%20Reference) (OtherBodyIndex :type Integer) (bFromSweep :type Boolean) (SweepResult :type Hit%20Result%20Structure%20%28by%20ref%29))
  (if (== (Variables|Default|GetPuzzlePiece2) (Utilities|GetClass OtherActor))
    (bind _asbp_master_item (Utilities|Casting|CastToBP_MasterItem OtherActor))
    (Transformation|SetActorLocation _asbp_master_item (Transformation|GetWorldLocation (Variables|Default|GetScene1)) false true)
    (Default|LockItem _asbp_master_item)
    (Default|PuzzlePieceSolved _asbp_master_item)))

(event OnComponentBeginOverlap(Check3)
  (params (OverlappedComponent :type Primitive%20Component%20Object%20Reference) (OtherActor :type Actor%20Object%20Reference) (OtherComp :type Primitive%20Component%20Object%20Reference) (OtherBodyIndex :type Integer) (bFromSweep :type Boolean) (SweepResult :type Hit%20Result%20Structure%20%28by%20ref%29))
  (if (== (Variables|Default|GetPuzzlePiece3) (Utilities|GetClass OtherActor))
    (bind _asbp_master_item (Utilities|Casting|CastToBP_MasterItem OtherActor))
    (Transformation|SetActorLocation _asbp_master_item (Transformation|GetWorldLocation (Variables|Default|GetScene)) false true)
    (Default|LockItem _asbp_master_item)
    (Default|PuzzlePieceSolved _asbp_master_item)))

(event EventBeginPlay)

(event Collision|EventActorBeginOverlap
  (params (OtherActor :type Actor%20Object%20Reference)))

(event EventTick
  (params (DeltaSeconds :type Float%20%28single-precision%29)))

(fn ConstructionScript)