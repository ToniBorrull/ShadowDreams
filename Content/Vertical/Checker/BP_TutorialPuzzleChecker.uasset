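; BP_TutorialPuzzleChecker is the final tutorial puzzle checker that detects a correct piece and completes the level.
; When an actor of the PuzzlePiece1 class overlaps Check1, it casts it to BP_MasterItem, teleports it onto Scene2 with zeroed rotation, locks it and marks it solved.
; Each solved piece increments ItemCount, and reaching TotalItemsToWin prints a win message and opens the Metro2 level.
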(event OnComponentBeginOverlap(Check1)
  (params (OverlappedComponent :type Primitive%20Component%20Object%20Reference) (OtherActor :type Actor%20Object%20Reference) (OtherComp :type Primitive%20Component%20Object%20Reference) (OtherBodyIndex :type Integer) (bFromSweep :type Boolean) (SweepResult :type Hit%20Result%20Structure%20%28by%20ref%29))
  ;[0.1367 0.8802 1] Comprobación Puzzle final
  (if (== (Variables|Default|GetPuzzlePiece1) (Utilities|GetClass OtherActor))
    (bind _asbp_master_item (Utilities|Casting|CastToBP_MasterItem OtherActor))
    (Transformation|SetActorLocation _asbp_master_item (Transformation|GetWorldLocation (Variables|Default|GetScene2)) false true)
    (Transformation|SetActorRotation _asbp_master_item "0, 0, 0" true)
    (Default|LockItem _asbp_master_item)
    (Default|PuzzlePieceSolved _asbp_master_item)
    (Development|PrintString "Piece1")
    (CallFunction|ItemDone)))

(event Custom|ItemDone
  (bind _itemcount (Variables|Default|GetItemCount))
  (Math|Integer|IncrementInt _itemcount
    (:%20%20
      (if (>= _itemcount (Variables|Default|GetTotalItemsToWin))
        (Development|PrintString "You WIn!")
        (Game|OpenLevel(byName) "Metro2")))))

(fn ConstructionScript)