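; BP_CheckPosition is a trigger volume that detects puzzle items and tells the first-person character when solving is possible.
; When a Puzzle1 or Puzzle2 class actor enters the box, it calls CanRotateOn, moves the physics handle target to its Scene component and sets CanSolve.
; Other overlaps switch FocusLight off.
; End overlap switches it on, clearing CanSolve only for non-matching actors.
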(event OnComponentBeginOverlap(Box)
  (params (OverlappedComponent :type Primitive%20Component%20Object%20Reference) (OtherActor :type Actor%20Object%20Reference) (OtherComp :type Primitive%20Component%20Object%20Reference) (OtherBodyIndex :type Integer) (bFromSweep :type Boolean) (SweepResult :type Hit%20Result%20Structure%20%28by%20ref%29))
  (bind _returnvalue (Utilities|GetClass OtherActor))
  ;[0.2648 0.05415 1] Item Detection
  (if (or (== (Variables|Default|GetPuzzle1) _returnvalue) (== _returnvalue (Variables|Default|GetPuzzle2)))
    (bind _asbp_first_person_character (Utilities|Casting|CastToBP_FirstPersonCharacter (Game|GetPlayerCharacter 0)))
    (Default|CanRotateon _asbp_first_person_character)
    (Physics|Components|PhysicsHandle|SetTargetLocation (Variables|/Game/Vertical/Player/BP_FirstPersonCharacter.BP_FirstPersonCharacter_C|GetPhysicsHandle _asbp_first_person_character) (Transformation|GetWorldLocation (Variables|Default|GetScene)))
    (Variables|/Game/Vertical/Player/BP_FirstPersonCharacter.BP_FirstPersonCharacter_C|SetcanSolve _asbp_first_person_character true)
    (else
      (Default|LightOff (Variables|Default|GetFocusLight) 1e+01))))

(event OnComponentEndOverlap(Box)
  (params (OverlappedComponent :type Primitive%20Component%20Object%20Reference) (OtherActor :type Actor%20Object%20Reference) (OtherComp :type Primitive%20Component%20Object%20Reference) (OtherBodyIndex :type Integer))
  (bind _focuslight (Variables|Default|GetFocusLight))
  ;[0.2648 0.05415 1] Item Detection
  (if (or (== (Variables|Default|GetPuzzle1) (Utilities|GetClass (stale OnComponentBeginOverlap(Box) OtherActor))) (== (Utilities|GetClass (stale OnComponentBeginOverlap(Box) OtherActor)) (Variables|Default|GetPuzzle2)))
    (Default|Lighton _focuslight false)
    (else
      (bind _asbp_first_person_character (Utilities|Casting|CastToBP_FirstPersonCharacter (Game|GetPlayerCharacter 0)))
      (Default|Lighton _focuslight true)
      (Variables|/Game/Vertical/Player/BP_FirstPersonCharacter.BP_FirstPersonCharacter_C|SetcanSolve _asbp_first_person_character false))))

(fn ConstructionScript)