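; Modular building actor that assembles a building from instanced Base, Body and Top modules in its Construction Script.
; Body copies stack above the base at intervals from mesh bounds and a vertical floor scale, with the top placed using the same offsets.
; It applies main and roof materials, driving UV layout and wall color variation through Custom Primitive Data.
; Informational strings report body story count and total height with and without roof elements.
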(event EventBeginPlay)

(event Collision|EventActorBeginOverlap
  (params (OtherActor :type Actor%20Object%20Reference)))

(event EventTick
  (params (DeltaSeconds :type Float%20%28single-precision%29)))

(fn ConstructionScript
  (bind _floor_height__bodymodulescale_ (Variables|Default|GetFloor%20Height%20%28BodyModuleScale%29))
  (bind _body_module (Variables|Default|GetBody_Module))
  (bind _max (Components|StaticMesh|GetLocalBounds _body_module))
  (bind _z (Math|Vector|BreakVector _max))
  (Rendering|Material|SetMaterial (Variables|Default|GetBase_Module) 0 (Variables|Default|GetMaterial_Main)) ; Sets Material for Building Modules\n(Base, Body and Top)
  (Rendering|Material|SetCustomPrimitiveDataFloat (Variables|Default|GetBody_Module) 0 (Variables|Default|GetUV_Layout_Selection)) ; Changes UVs Layouts of Building Modules\nControls the "TexCoor Index" parameter in the material, \npreviously set up as "Use Custom Primitive Data"
  (Rendering|Material|SetCustomPrimitiveDataFloat (Variables|Default|GetBody_Module) 1 (Variables|Default|GetWallsBetweenWindows_Switch)) ; Controls whether the color variation of the walls between windows\nis applied vertically or horizontally
  (Rendering|Material|SetMaterial (Variables|Default|GetTop_Module) 1 (Variables|Default|GetMaterial_RoofElements)) ; Sets material for Roof Elements
  (Components|InstancedStaticMesh|AddInstance (Variables|Default|GetBase_Module) (Math|Transform|MakeTransform "0, 0, 0" "0, 0, 0" "1.000000,1.000000,1.000000") false) ; Adds Base Module of Building
  (for _index (range 0 (Variables|Default|GetBody_Module_Copies)) ; Loop for adding copies of Body Module
    (Components|InstancedStaticMesh|AddInstance (Variables|Default|GetBody_Module) (Math|Transform|MakeTransform (Math|Vector|MakeVector 0.0 0.0 (+ (* (Math|Conversions|ToFloat(Integer) _index) (* _z _floor_height__bodymodulescale_)) (.Z (Math|Vector|BreakVector (.Max (Components|StaticMesh|GetLocalBounds (Variables|Default|GetBase_Module))))))) "0, 0, 0" (Math|Vector|MakeVector 1.0 1.0 _floor_height__bodymodulescale_)) false) ; Adds Copy of Body Module
  )
  (Components|InstancedStaticMesh|AddInstance (Variables|Default|GetTop_Module) (Math|Transform|MakeTransform (Math|Vector|MakeVector 0.0 0.0 (+ (* (Math|Conversions|ToFloat(Integer) _index) (* _z _floor_height__bodymodulescale_)) (.Z (Math|Vector|BreakVector (.Max (Components|StaticMesh|GetLocalBounds (Variables|Default|GetBase_Module))))))) "0, 0, 0" "1.000000,1.000000,1.000000") false) ; Adds Top Module of Building
  ;[0.2188 0.2188 0.2188] Informational Nodes Only - Can be deleted without afecting Construction of Building
  (Variables|BuildingSpecs(Informationalonly,noteditable)|SetNumber%20of%20Stories%20%28Body%20Module%20Only%29 (Utilities|String|ToString(Integer) (Math|Float|Round (* (/ (/ _z 1e+02) (Variables|Default|GetStandard_FloorHeight_%284m%29)) (+ (Variables|Default|GetBody_Module_Copies) 1)))))
  (Variables|BuildingSpecs(Informationalonly,noteditable)|SetTotalHeight_%28Meters%29 (Utilities|String|ToString(Integer) (Math|Float|Round (/ (+ (+ (* (Math|Conversions|ToFloat(Integer) _index) (* _z _floor_height__bodymodulescale_)) (.Z (Math|Vector|BreakVector (.Max (Components|StaticMesh|GetLocalBounds (Variables|Default|GetBase_Module)))))) (.Z (Math|Vector|BreakVector (.Max (Components|StaticMesh|GetLocalBounds (Variables|Default|GetTop_Module)))))) 1e+02))))
  (Variables|BuildingSpecs(Informationalonly,noteditable)|SetHeight_%28Without_RoofElements%29 (Utilities|String|ToString(Integer) (Math|Float|Round (/ (+ (+ (* (Math|Conversions|ToFloat(Integer) _index) (* _z _floor_height__bodymodulescale_)) (.Z (Math|Vector|BreakVector (.Max (Components|StaticMesh|GetLocalBounds (Variables|Default|GetBase_Module)))))) (.Z (Math|Vector|BreakVector (.Max (Components|StaticMesh|GetLocalBounds (Variables|Default|GetTop_Empty_Module)))))) 1e+02)))))