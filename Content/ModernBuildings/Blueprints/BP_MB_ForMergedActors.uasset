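; BP_MB_ForMergedActors is a modern-building Blueprint that displays a merged building mesh with configurable materials and variations.
; Its construction script assigns the main and roof-element materials to separate slots, then adds a mesh instance.
; Custom Primitive Data floats drive the material's UV layout selection and switch wall color variation between vertical and horizontal.
; All logic runs at construction; the event graph is empty.
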(event EventBeginPlay)

(event Collision|EventActorBeginOverlap
  (params (OtherActor :type Actor%20Object%20Reference)))

(event EventTick
  (params (DeltaSeconds :type Float%20%28single-precision%29)))

(fn ConstructionScript
  (bind _merged_actor_mesh (Variables|Default|GetMerged_Actor_Mesh))
  (Rendering|Material|SetMaterial _merged_actor_mesh 0 (Variables|Default|GetMaterial_Main)) ; Sets Material for Building
  (Rendering|Material|SetCustomPrimitiveDataFloat _merged_actor_mesh 0 (Variables|Default|GetUV_Layout_Selection)) ; Changes UVs Layouts of Building Modules\nControls the "TexCoor Index" parameter in the material, \npreviously set up as "Use Custom Primitive Data"
  (Rendering|Material|SetCustomPrimitiveDataFloat (Variables|Default|GetMerged_Actor_Mesh) 1 (Variables|Default|GetWallsBetweenWindows_Switch)) ; Controls whether the color variation of the walls between windows\nis applied vertically or horizontally
  (Rendering|Material|SetMaterial (Variables|Default|GetMerged_Actor_Mesh) 1 (Variables|Default|GetMaterial_RoofElements)) ; Sets material for Roof Elements
  (Components|InstancedStaticMesh|AddInstance (Variables|Default|GetMerged_Actor_Mesh) (Math|Transform|MakeTransform "0, 0, 0" "0, 0, 0" "1.000000,1.000000,1.000000") false) ; Adds mesh
)